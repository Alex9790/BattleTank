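; Player tank pawn Blueprint that binds input to driving, camera aiming and firing.
; BeginPlay hands the barrel and turret to the TankAiming component and both tracks to TankMovement.
; Per-track throttle and turn axes all feed shared forward, turn-right and turn-left intents on TankMovement, rather than driving tracks individually.
; Aim axes rotate an azimuth gimbal and spring arm separately for the camera, while Fire calls TankAiming.
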(event EventBeginPlay
  (Class|TankAimingComponent|Initialise (Variables|Default|GetTankAiming) (Variables|Default|GetTankBarrel2) (Variables|Default|GetTankTurret1))
  (Class|TankMovementComponent|Initialise (Variables|Default|GetTankMovement) (Variables|Default|GetLeftTrack) (Variables|Default|GetRightTrack)))

(event Collision|EventActorBeginOverlap
  (params (OtherActor :type Actor%20Object%20Reference)))

(event EventTick
  (params (DeltaSeconds :type Float%20%28single-precision%29)))

(event Input|ActionEvents|InputActionFire
  (params (Key :type Key%20Structure))
  ;[1 1 1] Input Mouse
  (:Pressed
    (Class|TankAimingComponent|Fire (Variables|Default|GetTankAiming))))

(event Input|AxisEvents|InputAxisAimAzimuth
  (params (AxisValue :type Float%20%28single-precision%29))
  ;[1 1 1] Camera Input Binding
  (Transformation|AddLocalRotation (Variables|Default|GetAzimuth%20Gimbal) (Math|Rotator|MakeRotator 0.0 0.0 AxisValue) false false))

(event Input|AxisEvents|InputAxisLeftTrackThrottleForward
  (params (AxisValue :type Float%20%28single-precision%29))
  ;[1 1 1] Movimiento del Tanque
  (Class|TankMovementComponent|IntendMoveForward (Variables|Default|GetTankMovement) AxisValue))

(event Input|AxisEvents|InputAxisAimElevation
  (params (AxisValue :type Float%20%28single-precision%29))
  ;[1 1 1] Camera Input Binding
  (Transformation|AddLocalRotation (Variables|Default|GetSpringArm) (Math|Rotator|MakeRotator 0.0 AxisValue 0.0) false false))

(event Input|AxisEvents|InputAxisLeftTrackTurnRight
  (params (AxisValue :type Float%20%28single-precision%29))
  ;[1 1 1] Movimiento del Tanque
  (Class|TankMovementComponent|IntendTurnRight (Variables|Default|GetTankMovement) AxisValue))

(event Input|AxisEvents|InputAxisLeftTrackTurnRight
  (params (AxisValue :type Float%20%28single-precision%29))
  ;[1 1 1] Movimiento del Tanque
  (Class|TankMovementComponent|IntendTurnRight (Variables|Default|GetTankMovement) AxisValue))

(event Input|AxisEvents|InputAxisLeftTrackThrottleBackward
  (params (AxisValue :type Float%20%28single-precision%29))
  ;[1 1 1] Movimiento del Tanque
  (Class|TankMovementComponent|IntendMoveForward (Variables|Default|GetTankMovement) AxisValue))

(event Input|AxisEvents|InputAxisRightTrackThrottleBackward
  (params (AxisValue :type Float%20%28single-precision%29))
  ;[1 1 1] Movimiento del Tanque
  (Class|TankMovementComponent|IntendMoveForward (Variables|Default|GetTankMovement) AxisValue))

(event Input|AxisEvents|InputAxisRightTrackThrottleForward
  (params (AxisValue :type Float%20%28single-precision%29))
  ;[1 1 1] Movimiento del Tanque
  (Class|TankMovementComponent|IntendMoveForward (Variables|Default|GetTankMovement) AxisValue))

(event Input|AxisEvents|InputAxisLeftTrackTurnLeft
  (params (AxisValue :type Float%20%28single-precision%29))
  ;[1 1 1] Movimiento del Tanque
  (Class|TankMovementComponent|IntendTurnLeft (Variables|Default|GetTankMovement) AxisValue))

(event Input|AxisEvents|InputAxisRightTrackTurnLeft
  (params (AxisValue :type Float%20%28single-precision%29))
  ;[1 1 1] Movimiento del Tanque
  (Class|TankMovementComponent|IntendTurnLeft (Variables|Default|GetTankMovement) AxisValue))

(fn ConstructionScript)